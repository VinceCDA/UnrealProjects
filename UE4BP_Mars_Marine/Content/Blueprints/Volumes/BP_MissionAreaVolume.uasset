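; BP_MissionAreaVolume is a volume that keeps the player inside the mission area and punishes leaving it.
; When a BP_Marine stops overlapping, it flags that marine as outside and starts a timer of DeathTimer seconds.
; Re-entering clears the flag and cancels the timer.
; If the timer expires, Kill Player applies 100 damage to player character 0, not necessarily the marine that left.
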(event EventBeginPlay)

(event EventTick
  (params (DeltaSeconds :type Float%20%28single-precision%29)))

(event Collision|EventActorBeginOverlap
  (params (OtherActor :type Actor%20Object%20Reference))
  ;[1 1 1] Player Entering Zone
  (bind _asbp_marine (Utilities|Casting|CastToBP_Marine OtherActor))
  (Variables|/Game/Blueprints/Pawns/BP_Marine.BP_Marine_C|SetOutside%20Mission%20Area _asbp_marine false)
  (Utilities|Time|ClearTimerbyFunctionName 0 "Kill Player"))

(event Collision|EventActorEndOverlap
  (params (OtherActor :type Actor%20Object%20Reference))
  ;[1 1 1] Player Leaving Zone
  (bind _asbp_marine (Utilities|Casting|CastToBP_Marine OtherActor))
  (Variables|/Game/Blueprints/Pawns/BP_Marine.BP_Marine_C|SetOutside%20Mission%20Area _asbp_marine true)
  (Utilities|Time|SetTimerbyFunctionName 0 "Kill Player" (Variables|Default|GetDeath%20Timer)))

(fn ConstructionScript)

(fn KillPlayer
  (Game|Damage|ApplyDamage (Game|GetPlayerCharacter 0) 1e+02 0 0))