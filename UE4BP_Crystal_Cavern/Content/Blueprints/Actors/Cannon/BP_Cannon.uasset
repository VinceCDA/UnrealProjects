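; BP_Cannon is a cannon actor that repeatedly fires projectiles on its own, starting at BeginPlay.
; After each fire-rate delay it spawns a BP_Projectile at the spawn point, using a configurable scale.
; It then plays a timeline that animates the barrel along its relative Y axis.
; The timeline's Cannon Fired event track restarts the delay, closing the firing loop without Tick.
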(event EventBeginPlay
  (Utilities|FlowControl|Delay (Variables|CannonProperties|GetCannon%20Fire%20Rate) :!label _label)
  (CallFunction|SpawnProjectiles)
  (bind _cannon_barrel_location (Timeline|Fire%20Cannon%20Timeline PlayFromStart)
    (:Update
      (CallFunction|MoveCannonBarrel _cannon_barrel_location))
    (:Cannon%20Fired
      (goto _label))))

(event Collision|EventActorBeginOverlap
  (params (OtherActor :type Actor%20Object%20Reference)))

(event EventTick
  (params (DeltaSeconds :type Float%20%28single-precision%29)))

(fn ConstructionScript)

(fn SpawnProjectiles
  (bind _projectile_spawn_point (Variables|Default|GetProjectile%20Spawn%20Point))
  (bind _returnvalue (Transformation|GetWorldTransform _projectile_spawn_point))
  (Game|SpawnActorfromClass "/Game/Blueprints/Actors/Projectiles/BP_Projectile.BP_Projectile_C" (Math|Transform|MakeTransform (.location _returnvalue) (.rotation _returnvalue) (Math|Conversions|ToVector(Float) (Variables|CannonProperties|GetProjectile%20Scale))) "AdjustIfPossibleButAlwaysSpawn" 0 0))

(fn MoveCannonBarrel
  (params (Cannon%20Barrel%20Y%20Location :type Float%20%28single-precision%29))
  (Transformation|SetRelativeLocation (Variables|Default|GetCannon_Barrel) (Math|Vector|MakeVector 0.0 Cannon%20Barrel%20Y%20Location 0.0) false false))